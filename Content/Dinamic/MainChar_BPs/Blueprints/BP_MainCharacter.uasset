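; Player character Blueprint for a shooter, handling Enhanced Input movement, a starting machine gun component, aim zoom, shell ejection and landing camera shakes.
; Jumping and sprinting spend stamina, with delayed self-calling events draining it during a sprint and refilling it afterwards.
; Recoil plays a timeline into controller pitch and yaw, then reverses it on stop, scaling recovery by pitch drift between the stored original and post-recoil rotations.
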(event `self.ReceiveBeginPlay`
  ;[0.2052 0.182 0] Connect basic movements
  (`EnhancedInputSubsystemInterface.AddMappingContext` (pcsubsystem `EnhancedInputLocalPlayerSubsystem` (`GameplayStatics.GetPlayerController` 0)) "/Game/Dinamic/MainChar_BPs/Basic_Movements/MC_BasicMovement.MC_BasicMovement" 0 (struct))
  ;[0 0.03924 1] Add gun at the start of game
  (bind _returnvalue (`|AddComponentByClass` "/Game/Dinamic/Guns_BPs/Machine_Gun/SMC_MachineGun.SMC_MachineGun_C"))
  (set `self.CurrentGun` _returnvalue))

(event `EnhancedInput|/Game/Dinamic/MainChar_BPs/Basic_Movements/IA_Jump`
  (params (ActionValue :type Boolean) (ElapsedSeconds :type "Float (double-precision)") (TriggeredSeconds :type "Float (double-precision)") (InputAction :type "InputAction Object Reference" :default "/Game/Dinamic/MainChar_BPs/Basic_Movements/IA_Jump.IA_Jump"))
  ;[0.2177 0.1853 0] Actors jump
  (:`Started`
    (`self.Jump`)
    (set `self.Stamina` (`KismetMathLibrary.Clamp` (- (`self.Stamina`) 25) 0 (`self.MaxStamina`))))
  (:`Completed`
    (`self.StopJumping`)))

(event `EnhancedInput|/Game/Dinamic/MainChar_BPs/Basic_Movements/IA_MoveForBack`
  (params (ActionValue :type "Float (double-precision)") (ElapsedSeconds :type "Float (double-precision)") (TriggeredSeconds :type "Float (double-precision)") (InputAction :type "InputAction Object Reference" :default "/Game/Dinamic/MainChar_BPs/Basic_Movements/IA_MoveForBack.IA_MoveForBack"))
  ;[0.3135 0.256 0] Move Actor Forward & Backward
  (:`Triggered`
    (`self.AddMovementInput` (`self.GetActorForwardVector`) ActionValue)))

(event `EnhancedInput|/Game/Dinamic/MainChar_BPs/Basic_Movements/IA_MoveRightLeft`
  (params (ActionValue :type "Float (double-precision)") (ElapsedSeconds :type "Float (double-precision)") (TriggeredSeconds :type "Float (double-precision)") (InputAction :type "InputAction Object Reference" :default "/Game/Dinamic/MainChar_BPs/Basic_Movements/IA_MoveRightLeft.IA_MoveRightLeft"))
  ;[0.376 0.314 0] Move Actor Right & Left
  (:`Triggered`
    (`self.AddMovementInput` (`self.GetActorRightVector`) ActionValue)))

(event `EnhancedInput|/Game/Dinamic/MainChar_BPs/Basic_Movements/IA_Pitch`
  (params (ActionValue :type "Float (double-precision)") (ElapsedSeconds :type "Float (double-precision)") (TriggeredSeconds :type "Float (double-precision)") (InputAction :type "InputAction Object Reference" :default "/Game/Dinamic/MainChar_BPs/Basic_Movements/IA_Pitch.IA_Pitch"))
  ;[0.376 0.3152 0] Pitch of the character
  (:`Triggered`
    (`self.AddControllerPitchInput` ActionValue)))

(event `EnhancedInput|/Game/Dinamic/MainChar_BPs/Basic_Movements/IA_Yaw`
  (params (ActionValue :type "Float (double-precision)") (ElapsedSeconds :type "Float (double-precision)") (TriggeredSeconds :type "Float (double-precision)") (InputAction :type "InputAction Object Reference" :default "/Game/Dinamic/MainChar_BPs/Basic_Movements/IA_Yaw.IA_Yaw"))
  ;[0.376 0.3152 0] Pitch of the character
  (:`Triggered`
    (`self.AddControllerYawInput` ActionValue)))

(event `EnhancedInput|/Game/Dinamic/MainChar_BPs/Basic_Movements/IA_Sprint`
  (params (ActionValue :type Boolean) (ElapsedSeconds :type "Float (double-precision)") (TriggeredSeconds :type "Float (double-precision)") (InputAction :type "InputAction Object Reference" :default "/Game/Dinamic/MainChar_BPs/Basic_Movements/IA_Sprint.IA_Sprint"))
  ;[0.09371 1 0] Sprinting
  (:`Started`
    (`self.Sprinting` ActionValue))
  (:`Completed`
    (`self.StopSprinting`)))

(event `ToggleAimView`
  ;[0.08305 1 0] Toggle aim view
  (bind _output_get (set `self.IsAiming?` (`/Game/Dinamic/Guns_BPs/Pistol/SMC_Pistol.IsAiming` (cast `/Game/Dinamic/Guns_BPs/Pistol/SMC_Pistol` (`self.CurrentGun`) :!pure true))))
  (if _output_get
    (bind (_direction _aimvalue _addaimvalue) (`Timeline|Timeline` :!label _label)
      (:`Update`
        (set `self.AddSpread` _addaimvalue)
        (`CameraComponent.SetFieldOfView` (`self.Camera`) (`KismetMathLibrary.Lerp` 90.0 70.0 _aimvalue))))
    (else
      (goto _label :!via `Reverse`))))

(event `self.OnLanded`
  (params (Hit :type "HitResult Structure (by ref)"))
  (bind _returnvalue (`self.K2_GetActorLocation`))
  (bind (_returnvalue_x _returnvalue_y _returnvalue_z) (`KismetMathLibrary.BreakVector` (`self.GetVelocity`)))
  ;[0 1 0.005693] Landing camera shake
  (if (< _returnvalue_z -1000.0)
    (`GameplayStatics.PlayWorldCameraShake` "/Game/Dinamic/MainChar_BPs/CameraShakes/HighJump_Shake.HighJump_Shake_C" _returnvalue 0.0 3000.0)
    (else
      (`GameplayStatics.PlayWorldCameraShake` "/Game/Dinamic/MainChar_BPs/CameraShakes/Jump_Shake.Jump_Shake_C" _returnvalue 0.0 3000.0))))

(event `SpawnShell`
  ;[0 0.6827 1] Spawning pistol shell
  (bind _returnvalue (`|SpawnActorFromClass` (`self.TypeOfShell`) (`SceneComponent.GetSocketTransform` (`self.CurrentGun`) "Shells_Place" "RTS_World") "AlwaysSpawn" "MultiplyWithRoot" null null))
  (bind _asbp_pistol_ammo (cast `/Game/Dinamic/Ammo_BPs/BP_PistolAmmo` _returnvalue))
  (bind _shell (`/Game/Dinamic/Ammo_BPs/BP_PistolAmmo.Shell` _asbp_pistol_ammo))
  (`PrimitiveComponent.SetSimulatePhysics` _shell true)
  (`PrimitiveComponent.AddImpulse` _shell (+ (* (`SceneComponent.GetForwardVector` _shell) (`KismetMathLibrary.RandomFloatInRange` 1.0 5.0)) (* (`SceneComponent.GetRightVector` _shell) (`KismetMathLibrary.RandomFloatInRange` 1.0 5.0))) "None" false)
  (`KismetSystemLibrary.Delay` 2.5)
  (`self.K2_DestroyActor` _returnvalue))

(event `SpendStamina`
  (bind _output_get (set `self.Stamina` (`KismetMathLibrary.Clamp` (- (`self.Stamina`) 5) 0 (`self.MaxStamina`))))
  (if (== _output_get 0)
    (`self.StopSprinting`)
    (elif (and (`self.IsRunning`) (> (`KismetMathLibrary.VSize` (`self.GetVelocity`)) 200.0))
      (`KismetSystemLibrary.Delay` 0.5)
      (`KismetSystemLibrary.PrintString` (`KismetStringLibrary.Conv_IntToString` (`self.Stamina`)))
      (`self.SpendStamina`))))

(event `GainStamina`
  (bind _output_get (set `self.Stamina` (`KismetMathLibrary.Clamp` (+ (`self.Stamina`) 5) 0 (`self.MaxStamina`))))
  (`KismetSystemLibrary.PrintString` (`KismetStringLibrary.Conv_IntToString` (`self.Stamina`)))
  (if (== _output_get (`self.MaxStamina`))
    _
    (elif (not (`self.IsRunning`))
      (`KismetSystemLibrary.Delay` 0.4)
      (`self.GainStamina`))))

(event `FireSpread`
  (bind _recoilmaxthreshold (`self.RecoilMaxThreshold`))
  (bind _returnvalue (`KismetMathLibrary.Abs` (.pitch (`KismetMathLibrary.NormalizedDeltaRotator` (`self.OriginRotation`) (`self.PostRecoil`)))))
  (bind _returnvalue_2 (`KismetMathLibrary.SelectFloat` (`KismetMathLibrary.MapRangeClamped` _returnvalue 0.0 _recoilmaxthreshold 0.0 1.0) (`KismetMathLibrary.MapRangeClamped` _returnvalue _recoilmaxthreshold 30.0 1.0) (> _returnvalue (`self.RecoilMaxThreshold`))))
  ;[0 0.6157 1] PistolSpread
  (`TimelineComponent.SetPlayRate` (`self.Spread_Pistol`) 1.0)
  (`|ExecutionSequence`
    (:`then_0`
      (`/Engine/EditorBlueprintResources/StandardMacros.DoOnce` false :!label _label
        (:`Completed`
          (set `self.OriginRotation` (`Controller.GetControlRotation` (`GameplayStatics.GetPlayerController` 0))))))
    (:`then_1`
      (bind (_direction _pitchinput _yawinput) (`Timeline|Spread_Pistol` :!label _label_2)
        (:`Update`
          (switch `ETimelineDirection` _direction
            (:`Forward`
              (`self.SpreadMoveGun` _pitchinput _yawinput))
            (:`Backward`
              (`|ExecutionSequence`
                (:`then_0`
                  (`/Engine/EditorBlueprintResources/StandardMacros.DoOnce` false :!label _label_3
                    (:`Completed`
                      (set `self.PostRecoil` (`Controller.GetControlRotation` (`GameplayStatics.GetPlayerController` 0))))))
                (:`then_1`
                  (`self.SpreadMoveGun` (* _pitchinput -6.0 _returnvalue_2) (* _yawinput -3.0 _returnvalue_2)))))))
        (:`Finished`
          (switch `ETimelineDirection` _direction
            (:`Backward`
              (`self.CE_ResetRecoil`))))))))

(event `CE_ResetRecoil`
  ;[0 0.6157 1] PistolSpread
  (`|ExecutionSequence`
    (:`then_0`
      (goto _label :!via `Reset`))
    (:`then_1`
      (goto _label_3 :!via `Reset`))))

(event `FireStopSpread`
  ;[0 0.6157 1] PistolSpread
  (`TimelineComponent.SetPlayRate` (`self.Spread_Pistol`) 6.0)
  (goto _label_2 :!via `Reverse`))

(fn `Sprinting`
  (params (IsSprinting :type Boolean))
  (if (and (not (`NavMovementComponent.IsFalling` (`self.CharacterMovement`))) IsSprinting (not (`self.IsAiming?`)))
    (set `self.IsRunning` true)
    (set `CharacterMovementComponent.MaxWalkSpeed` 400.0 (`self.CharacterMovement`))
    (`self.SpendStamina`)))

(fn `StopSprinting`
  (set `self.IsRunning` false)
  (set `CharacterMovementComponent.MaxWalkSpeed` 250.0 (`self.CharacterMovement`))
  (`self.GainStamina`))

(fn `UserConstructionScript`)